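; Ball actor that moves and bounces around the level while BallGameMode is outside its first game state.
; Each Tick it does a swept, planar move along Direction by a per-frame Speed, without delta-time scaling, and reflects off the impact normal.
; Paddle hits skew the bounce by the paddle's input axis and add a MinX bias.
; Other actors implementing BallHitInterface receive HitByBallMessage.
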(event EventBeginPlay)

(event Collision|EventActorBeginOverlap
  (params (OtherActor :type Actor%20Object%20Reference)))

(event EventTick
  (params (DeltaSeconds :type Float%20%28single-precision%29))
  (bind _asball_game_mode (Utilities|Casting|CastToBallGameMode (Game|GetGameMode)))
  (if (not (Utilities|Enum|Equal(Enum) (Variables|/Game/Blueprints/BallGameMode.BallGameMode_C|GetState%20of%20The%20Game _asball_game_mode) "NewEnumerator0"))
    (bind _sweephitresult (Transformation|AddActorWorldOffset (Math|Vector|MakeVector (.X (Math|Vector|BreakVector (* (Variables|Default|GetDirection) (Variables|Default|GetSpeed)))) (.Y (Math|Vector|BreakVector (* (Variables|Default|GetDirection) (Variables|Default|GetSpeed)))) 0.0) true))
    (bind _aspaddle (Utilities|Casting|CastToPaddle (.HitActor (Collision|BreakHitResult _sweephitresult)))
      (:then
        (Variables|Default|SetDirection (Math|Vector|Normalize (Math|Vector|MakeVector (+ (.X (Math|Vector|BreakVector (Math|Vector|Normalize (Math|Vector|MakeVector (.X (Math|Vector|BreakVector (Math|Vector|GetReflectionVector (Variables|Default|GetDirection) (.ImpactNormal (Collision|BreakHitResult _sweephitresult))))) (+ (* (Variables|/Game/Blueprints/Paddle.Paddle_C|GetAxis%20Value _aspaddle) 5.0) (.Y (Math|Vector|BreakVector (Math|Vector|GetReflectionVector (Variables|Default|GetDirection) (.ImpactNormal (Collision|BreakHitResult _sweephitresult)))))) (.Z (Math|Vector|BreakVector (Math|Vector|GetReflectionVector (Variables|Default|GetDirection) (.ImpactNormal (Collision|BreakHitResult _sweephitresult))))))))) (Variables|Default|GetMinX)) (.Y (Math|Vector|BreakVector (Math|Vector|Normalize (Math|Vector|MakeVector (.X (Math|Vector|BreakVector (Math|Vector|GetReflectionVector (Variables|Default|GetDirection) (.ImpactNormal (Collision|BreakHitResult _sweephitresult))))) (+ (* (Variables|/Game/Blueprints/Paddle.Paddle_C|GetAxis%20Value _aspaddle) 5.0) (.Y (Math|Vector|BreakVector (Math|Vector|GetReflectionVector (Variables|Default|GetDirection) (.ImpactNormal (Collision|BreakHitResult _sweephitresult)))))) (.Z (Math|Vector|BreakVector (Math|Vector|GetReflectionVector (Variables|Default|GetDirection) (.ImpactNormal (Collision|BreakHitResult _sweephitresult))))))))) (.Z (Math|Vector|BreakVector (Math|Vector|Normalize (Math|Vector|MakeVector (.X (Math|Vector|BreakVector (Math|Vector|GetReflectionVector (Variables|Default|GetDirection) (.ImpactNormal (Collision|BreakHitResult _sweephitresult))))) (+ (* (Variables|/Game/Blueprints/Paddle.Paddle_C|GetAxis%20Value _aspaddle) 5.0) (.Y (Math|Vector|BreakVector (Math|Vector|GetReflectionVector (Variables|Default|GetDirection) (.ImpactNormal (Collision|BreakHitResult _sweephitresult)))))) (.Z (Math|Vector|BreakVector (Math|Vector|GetReflectionVector (Variables|Default|GetDirection) (.ImpactNormal (Collision|BreakHitResult _sweephitresult)))))))))))))
      (:CastFailed
        (Variables|Default|SetDirection (Math|Vector|GetReflectionVector (Variables|Default|GetDirection) (.ImpactNormal (Collision|BreakHitResult _sweephitresult))))
        (if (Utilities|DoesObjectImplementInterface (.HitActor (Collision|BreakHitResult _sweephitresult)) "/Game/Blueprints/BallHitInterface.BallHitInterface_C")
          (Class|BallHitInterface|HitbyBall(Message) (.HitActor (Collision|BreakHitResult _sweephitresult))))))))

(fn ConstructionScript)