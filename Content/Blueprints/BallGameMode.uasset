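; BallGameMode is a game mode that holds the game's state and runs a three-second start countdown.
; BeginPlay sets the initial state, and StartCountdown resets the timer and switches to the countdown state.
; While in that state, Tick subtracts delta time, maps the remaining time to a whole-number Count of 3, 2 or 1, then advances the state once it drops below zero.
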(event Custom|StartCountdown
  ;[0.7916 1 0.2622] StartCountdown
  (Variables|Default|SetCountDown 3.0)
  (Variables|Default|SetState%20of%20The%20Game "NewEnumerator1"))

(event EventBeginPlay
  (Variables|Default|SetState%20of%20The%20Game "NewEnumerator0"))

(event EventTick
  (params (DeltaSeconds :type Float%20%28single-precision%29))
  (if (Utilities|Enum|Equal(Enum) (Variables|Default|GetState%20of%20The%20Game) "NewEnumerator1")
    (bind _output_get (Variables|Default|SetCountDown (- (Variables|Default|GetCountDown) DeltaSeconds)))
    (if (>= _output_get 2.0)
      (Variables|Default|SetCount 3)
      (elif (>= _output_get 1.0)
        (Variables|Default|SetCount 2)
        (elif (>= _output_get 0.0)
          (Variables|Default|SetCount 1)
          (else
            (Variables|Default|SetState%20of%20The%20Game "NewEnumerator5")))))))

(fn ConstructionScript)